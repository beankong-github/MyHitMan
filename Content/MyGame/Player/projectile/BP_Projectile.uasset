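; BP_Projectile is a projectile that delivers Gameplay Ability System effects to the actor it hits.
; When its Sphere component registers a hit, it calls DestroyActor first, then looks for an Ability System Component on the hit actor.
; If both that actor and the instigator have one, the instigator's component applies AttackEffect and HitTagEffect to the target.
; Destruction also prints a debug string.
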(event OnComponentHit(Sphere)
  (params (HitComponent :type Primitive%20Component%20Object%20Reference) (OtherActor :type Actor%20Object%20Reference) (OtherComp :type Primitive%20Component%20Object%20Reference) (NormalImpulse :type Vector :default "0, 0, 0") (Hit :type Hit%20Result%20Structure%20%28by%20ref%29))
  (bind _returnvalue (Game|GetInstigator))
  (bind _returnvalue_2 (Actor|GetComponentbyClass _returnvalue "/Script/GameplayAbilities.AbilitySystemComponent"))
  (Actor|DestroyActor)
  (bind _output_get (Variables|Default|SetOtherASC (Actor|GetComponentbyClass OtherActor "/Script/GameplayAbilities.AbilitySystemComponent")))
  (Utilities|IsValid _output_get
    (:Is%20Valid
      (Utilities|IsValid _returnvalue_2
        (:Is%20Valid
          (GameplayEffects|ApplyGameplayEffectToTarget :self _returnvalue_2 :GameplayEffectClass (Variables|Default|GetAttackEffect) :Target (Variables|Default|GetOtherASC))
          (GameplayEffects|ApplyGameplayEffectToTarget :self _returnvalue_2 :GameplayEffectClass (Variables|Default|GetHitTagEffect) :Target (Variables|Default|GetOtherASC)))))))

(event EventBeginPlay)

(event Collision|EventActorBeginOverlap
  (params (OtherActor :type Actor%20Object%20Reference)))

(event EventTick
  (params (DeltaSeconds :type Float%20%28single-precision%29)))

(event EventDestroyed
  (Development|PrintString "Projectile Destroyed"))

(fn ConstructionScript)