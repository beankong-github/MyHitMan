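; Mushroom monster Blueprint that wires its hit reaction through the Gameplay Ability System.
; BeginPlay runs the parent logic, binds a listener to the Player.State.Hit tag on its ASC, and grants the mushroom Dead and Hit abilities.
; When that tag's count is one, the listener activates the Hit ability by class.
; The Dead ability is only granted here, with no activation in this graph.
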(event Custom|On%20Tag%20changed
  (params (Tag :type Gameplay%20Tag%20Structure%20%28by%20ref%29) (TagCount :type Integer))
  (if (and (== TagCount 1) (GameplayTags|HasTag (GameplayTags|MakeGameplayTagContainerfromTag "(TagName=\"Player.State.Hit\")") Tag))
    (Abilities|TryActivateAbilitybyClass (Variables|Default|GetASC) "/Game/MyGame/ASC/GA/Monster/BPGA_MushroomHit.BPGA_MushroomHit_C" true)))

(event EventBeginPlay
  (|CallParentFunction)
  (GameplayTags|BindEventWrappertoGameplayTagChanged (Variables|Default|GetASC) "(TagName=\"Player.State.Hit\")" (delegate Custom|On%20Tag%20changed))
  (GameplayAbilities|GiveAbility (Variables|Default|GetASC) "/Game/MyGame/ASC/GA/Monster/BPGA_MushroomDead.BPGA_MushroomDead_C" 0 -1)
  (GameplayAbilities|GiveAbility (Variables|Default|GetASC) "/Game/MyGame/ASC/GA/Monster/BPGA_MushroomHit.BPGA_MushroomHit_C" 0 -1))

(fn ConstructionScript
  (|CallParentFunction))