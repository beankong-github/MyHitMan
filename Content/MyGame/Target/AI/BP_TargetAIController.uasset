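; AI controller for a target character that runs the BT_TargetAI behavior tree on possession.
; A perception update that senses a Player-tagged actor cancels the timer and writes HasLineOfSight and PlayerActor to the Blackboard.
; Any other update starts a LineOfSightTimer delay, after which both keys are cleared, giving a grace period before losing the player.
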(event OnTargetPerceptionUpdated(AIPerception)
  (params (Actor :type Actor%20Object%20Reference) (Stimulus :type AI%20Stimulus%20Structure))
  (bind _blackboard (Variables|Default|GetBlackboard))
  (if (and (Actor|ActorHasTag Actor "Player") (Utilities|Struct|BreakAIStimulus Stimulus))
    (Utilities|Time|ClearandInvalidateTimerbyHandle (Variables|Default|GetTimer))
    (AI|Components|Blackboard|SetValueasBool _blackboard (Variables|Default|GetHasLineOfSight) true)
    (AI|Components|Blackboard|SetValueasObject _blackboard (Variables|Default|GetPlayerActor) Actor)
    (else
      (bind _returnvalue (Utilities|Time|SetTimerbyEvent (delegate Custom|Start%20Enemy%20Timer) (Variables|Default|GetLine%20of%20Sight%20Timer)))
      (Variables|Default|SetTimer _returnvalue))))

(event Custom|Start%20Enemy%20Timer
  (bind _blackboard (Variables|Default|GetBlackboard))
  (AI|Components|Blackboard|SetValueasBool _blackboard (Variables|Default|GetHasLineOfSight) false)
  (AI|Components|Blackboard|SetValueasObject _blackboard (Variables|Default|GetPlayerActor) 0))

(event EventPossess
  (params (PossessedPawn :type Pawn%20Object%20Reference))
  (AI|RunBehaviorTree "/Game/MyGame/Target/AI/BT_TargetAI.BT_TargetAI"))

(fn ConstructionScript)